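; VR full-body player pawn that hides the mesh's head bone and headset model and exposes head, hand and elbow transforms as IK targets.
; Tick copies motion controller and elbow component transforms, turns the mesh to camera yaw with a 90-degree offset, and sets the camera to the stored head transform.
; The construction script seeds these targets for AnimBP preview and experimentally scales mesh height and shifts the origin to player height.
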(event Custom|Rotate%20mesh%20tick
  (Transformation|SetWorldRotation (Variables|Character|GetMesh) (Math|Rotator|MakeRotator 0.0 0.0 (Variables|IK/locomotion|GetRotation)) false false) ; rotate mesh to face camera direction when moving
)

(event EventBeginPlay
  (CallFunction|AlignMeshtoCameraRotation)
  (Components|SkinnedMesh|HideBonebyName (Variables|Character|GetMesh) "head" "PBO_None")
  (Development|SetHiddeninGame (Variables|Default|GetHMD) true false)
  (Class|HeadMountedDisplayFunctionLibrary|SetTrackingOrigin "Eye"))

(event Collision|EventActorBeginOverlap
  (params (OtherActor :type Actor%20Object%20Reference)))

(event EventTick
  (params (DeltaSeconds :type Float%20%28single-precision%29))
  (Utilities|FlowControl|Sequence
    (:then_1
      (CallFunction|SetElbowPosition))
    (:then_2
      (|UpdateHandPoses))
    (:then_3
      (CallFunction|AlignMeshtoCameraRotation))
    (:then_4
      (Transformation|SetWorldTransform (Variables|Default|GetCamera) (Variables|IK/locomotion|GetHead%20Pos) false false))))

(fn ConstructionScript
  ;[0.6302 0.2091 0] Set initial positions so animBP shows preview
  (Variables|IK/locomotion|SetIK%20Hand%20Pos%20L (Transformation|GetWorldTransform (Variables|Default|GetMotionController_L)))
  (Variables|IK/locomotion|SetIK%20Hand%20Pos%20R (Transformation|GetWorldTransform (Variables|Default|GetMotionController_R)))
  (CallFunction|SetHeadPosition)
  (CallFunction|SetElbowPosition)
  (CallFunction|ScaleCharacterandOriginHeight) ; 2.2.1: scale pawn height (experimental)
)

(fn AlignMeshtoCameraRotation
  (bind _mesh (Variables|Character|GetMesh))
  (bind _camera (Variables|Default|GetCamera))
  (bind _returnvalue (Transformation|GetWorldRotation _camera))
  (bind _returnvalue_2 (Transformation|GetWorldRotation _mesh))
  (bind _returnvalue_3 (- (.yaw _returnvalue) 9e+01))
  (Transformation|SetWorldRotation (Variables|Character|GetMesh) (Math|Rotator|MakeRotator (.roll _returnvalue_2) (.pitch _returnvalue_2) _returnvalue_3) false false) ; rotate mesh to face camera direction
  (Variables|IK/locomotion|SetRotation _returnvalue_3))

(fn SetHeadPosition
  (bind _camera (Variables|Default|GetCamera))
  (bind _output_get (Variables|IK/locomotion|SetHead%20Pos (Math|Transform|MakeTransform (- (Transformation|GetWorldLocation _camera) (* (Math|Vector|GetForwardVector _camera) (Variables|IK/locomotion|GetEye%20offset))) (Transformation|GetWorldRotation _camera) "1.000000,1.000000,1.000000")))
  (return _output_get))

(fn SetElbowPosition
  (Variables|IK/locomotion|SetElbow%20Pos%20L (Transformation|GetWorldTransform (Variables|Default|GetElbow_L)))
  (Variables|IK/locomotion|SetElbow%20Pos%20R (Transformation|GetWorldTransform (Variables|Default|GetElbow_R))))

(fn ScaleCharacterandOriginHeight
  (bind _origin (Variables|Default|GetOrigin))
  (bind _relativelocation (Variables|/Script/Engine.SceneComponent|GetRelativeLocation _origin))
  (Transformation|SetWorldScale3D (Variables|Character|GetMesh) (Math|Vector|MakeVector 1.0 1.0 (/ (Variables|IK/locomotion|GetVRPlayerHeight) (Variables|IK/locomotion|GetCharacterMeshHeight))))
  (Transformation|SetRelativeLocation (Variables|Default|GetOrigin) (Math|Vector|MakeVector (.x _relativelocation) (.y _relativelocation) (+ (.z _relativelocation) (- (Variables|IK/locomotion|GetVRPlayerHeight) (Variables|IK/locomotion|GetCharacterMeshHeight)))) false false))

(fn UpdateHeadPosition
  (CallFunction|SetHeadPosition))