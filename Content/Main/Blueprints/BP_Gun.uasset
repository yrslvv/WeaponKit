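; VR handgun with a hand-racked slide, insertable magazines, trigger input, sounds and haptics.
; Slide grabs snap the hand mesh to the slide and use looping timers to clamp travel and ease it home; only Grip grabs update chambering.
; Type-matched held magazines snap into their socket on overlap.
; Holding the handle adds per-hand input mappings; firing checks round state, plays slide timelines and runs debug-drawn barrel traces.
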(event EventBeginPlay)

(event Collision|EventActorBeginOverlap
  (params (OtherActor :type Actor%20Object%20Reference)))

(event EventTick
  (params (DeltaSeconds :type Float%20%28single-precision%29)))

(event OnGrabbed(CurlGrabComponent)
  (params (Motion%20Controller :type Motion%20Controller%20Component%20Object%20Reference))
  ;[1 0.7919 0] In Development...
  (|AttachHandToSlide Motion%20Controller)
  (CallFunction|PlaySoundatLocation (Transformation|GetWorldLocation (Variables|Default|GetSlideGrabCollision)) (Variables|Sounds|GetSlideGrabSound))
  (Variables|SlideVariables|SetInitialGrabOffset (CallFunction|GetGrabOffsetBetweenMC&SlideCurl))
  (Utilities|Time|SetTimerbyEvent (delegate Custom|MoveGunSlideTowardsHand) 0.01 true))

(event OnDropped(GripGrabComponent)
  ;[0.005182 0.005182 0.005182] Slider Main Release Functionality
  (|AttachHandMeshToMotionConttroller&AddOffset_2) ; Alligns Hands With Where They Have To Be (see VRPawn)
  (Variables|Default|SetMotion%20Controller 0)
  (Variables|Default|SetMotionControllerHandMesh 0)
  (Class|KismetSystemLibrary|PauseTimer 0 "CustomEvent1")
  (if (<= (Variables|SlideVariables|GetCurrentSlideOffset) (Variables|Functionality|GetSlideOffsetToPlayAReleaseSound))
    ;;[0.3712 0.3712 0.3712] Play Release Effect
    (CallFunction|PlaySoundatLocation (Transformation|GetWorldLocation (Variables|Default|GetMuzzleMesh)) (Variables|Sounds|GetSlideReleased))
    (|PlayHapticEffectOnHandleHand) ; Slide Sends Vibration To Hand That Holds A Gun, therefore opposite
  )
  (Utilities|Time|SetTimerbyEvent (delegate Custom|CustomEvent) 0.01 true))

(event OnGrabbed(GripGrabComponent)
  (params (Motion%20Controller :type Motion%20Controller%20Component%20Object%20Reference))
  ;[0.005182 0.005182 0.005182] Slider Main Grip Functionality
  (|AttachHandToSlide_2 Motion%20Controller)
  (CallFunction|PlaySoundatLocation (Transformation|GetWorldLocation (Variables|Default|GetSlideGrabCollision)) (Variables|Sounds|GetSlideGrabSound))
  (Variables|SlideVariables|SetInitialGrabOffset (CallFunction|GetGrabOffsetBetweenMC&SlideDefault))
  (Utilities|Time|SetTimerbyEvent (delegate Custom|CustomEvent1) 0.01 true))

(event OnDropped(CurlGrabComponent)
  ;[1 0.7919 0] In Development...
  (|AttachHandMeshToMotionConttroller&AddOffset) ; Alligns Hands With Where They Have To Be (see VRPawn)
  (Variables|Default|SetMotion%20Controller 0)
  (Variables|Default|SetMotionControllerHandMesh 0)
  (Class|KismetSystemLibrary|PauseTimer 0 "MoveGunSlideTowardsHand")
  (if (<= (Variables|SlideVariables|GetCurrentSlideOffset) (Variables|Functionality|GetSlideOffsetToPlayAReleaseSound))
    ;;[0.01562 0.01562 0.01562] Play Release Effect
    (CallFunction|PlaySoundatLocation (Transformation|GetWorldLocation (Variables|Default|GetMuzzleMesh)) (Variables|Sounds|GetSlideReleased))
    (|PlayHapticEffectOnOppositeHand) ; Slide Sends Vibration To Hand That Holds A Gun, therefore opposite
  )
  (Utilities|Time|SetTimerbyEvent (delegate Custom|MoveSliderTowardsOrigin) 0.01 true))

(event Custom|CustomEvent1
  (bind _charging_handle_max_distance (Variables|Functionality|GetCharging%20Handle%20Max%20Distance))
  (bind _returnvalue (CallFunction|ClampSlideMovementDefault _charging_handle_max_distance))
  ;[0.005182 0.005182 0.005182] Slider Main Grip Functionality
  (if (not (>= (Math|Vector|Distance(Vector) (Transformation|GetWorldLocation (Variables|Default|GetMotion%20Controller)) (Transformation|GetWorldLocation (Variables|Default|GetMotionControllerHandMesh))) (Variables|Default|GetMaxMCDistanceFromGunToRelease)))
    (if (and (== _returnvalue (Variables|Functionality|GetCharging%20Handle%20Max%20Distance)) (not (Variables|SlideVariables|GetReachedCockSound?)))
      ;;[0.3698 0.3698 0.3698] Play Slide Cock Sound
      (Variables|SlideVariables|SetReachedCockSound? true)
      (CallFunction|PlaySoundatLocation (Transformation|GetWorldLocation (Variables|Default|GetSlideGrabCollision)) (Variables|Sounds|GetSlideCockSound))
      (bind _magazine (Variables|Attachments|GetMagazine)
        (:then
          (if (Variables|/Game/Main/Blueprints/BP_Magazine.BP_Magazine_C|GetIsEmpty _magazine)
            (Variables|SlideVariables|SetDryFire true :!label _label)
            (Variables|SlideVariables|SetBulletIsReadyToBeTakenFromMag false)
            (else
              (Variables|SlideVariables|SetDryFire false)
              (Variables|SlideVariables|SetBulletIsReadyToBeTakenFromMag true))))
        (:else
          (goto _label)))
      (if (Variables|SlideVariables|GetChamberHasBullet)
        (|InitiateBulletThrowAndSetRoundMeshInvisible))
      (|PlayHapticEffectOnHoldingHand))
    (bind _output_get (Variables|SlideVariables|SetCurrentSlideOffset _returnvalue))
    (Transformation|SetRelativeLocation (Variables|Default|GetSlideMesh) (Math|Vector|MakeVector _output_get 0.0 0.0) false false)))

(event Custom|CustomEvent
  ;[0.005182 0.005182 0.005182] Slider Main Release Functionality
  (bind _returnvalue (|InterpolateMeshAndContinueOnceCloseToDestinationGC)) ; Interpolated SlideMesh To Origin And Returns True Once Close To It
  (if _returnvalue
    (Transformation|SetRelativeLocation (Variables|Default|GetSlideMesh) (Math|Vector|MakeVector 0.0 0.0 0.0) false false)
    (Class|KismetSystemLibrary|PauseTimer 0 "CustomEvent")
    (if (Variables|SlideVariables|GetReachedCockSound?)
      (bind _magazine (Variables|Attachments|GetMagazine)
        (:then
          (if (Variables|SlideVariables|GetBulletIsReadyToBeTakenFromMag)
            (if (Variables|/Game/Main/Blueprints/BP_Magazine.BP_Magazine_C|GetIsEmpty _magazine)
              (if (Variables|SlideVariables|GetChamberHasBullet)
                (Variables|SlideVariables|SetDryFire true :!label _label)
                (Rendering|SetVisibility (Variables|Default|GetRoundMesh) false false)
                (Variables|SlideVariables|SetChamberHasBullet false)
                (Variables|SlideVariables|SetReachedCockSound? false :!label _label_2))
              (else
                (Default|RemoveRound (Variables|Attachments|GetMagazine))
                (Rendering|SetVisibility (Variables|Default|GetRoundMesh) true false)
                (Variables|SlideVariables|SetChamberHasBullet true)
                (goto _label_2)))
            (else
              (Variables|SlideVariables|SetReachedCockSound? false :!label _label_3))))
        (:else
          (goto _label)))
      (else
        (goto _label_3)))))

(event Custom|MoveSliderTowardsOrigin
  ;[1 0.7919 0] In Development...
  (bind _returnvalue (|InterpolateMeshAndContinueOnceCloseToDestination)) ; Interpolated SlideMesh To Origin And Returns True Once Close To It
  (if _returnvalue
    (Transformation|SetRelativeLocation (Variables|Default|GetSlideMesh) (Math|Vector|MakeVector 0.0 0.0 0.0) false false)
    (Class|KismetSystemLibrary|PauseTimer 0 "MoveSliderTowardsOrigin")))

(event Custom|MoveGunSlideTowardsHand
  (bind _charging_handle_max_distance (Variables|Functionality|GetCharging%20Handle%20Max%20Distance))
  (bind _returnvalue (CallFunction|ClampSlideMovementCurl _charging_handle_max_distance))
  ;[1 0.7919 0] In Development...
  (if (not (>= (Math|Vector|Distance(Vector) (Transformation|GetWorldLocation (Variables|Default|GetMotion%20Controller)) (Transformation|GetWorldLocation (Variables|Default|GetMotionControllerHandMesh))) (Variables|Default|GetMaxMCDistanceFromGunToRelease)))
    (if (and (== _returnvalue (Variables|Functionality|GetCharging%20Handle%20Max%20Distance)) (not (Variables|SlideVariables|GetReachedCockSound?)))
      ;;[0.02604 0.02604 0.02604] Play Slide Cock Sound
      (Variables|SlideVariables|SetReachedCockSound? true)
      (CallFunction|PlaySoundatLocation (Transformation|GetWorldLocation (Variables|Default|GetSlideGrabCollision)) (Variables|Sounds|GetSlideCockSound))
      (|PlayHapticEffect))
    (bind _output_get (Variables|SlideVariables|SetCurrentSlideOffset _returnvalue))
    (Transformation|SetRelativeLocation (Variables|Default|GetSlideMesh) (Math|Vector|MakeVector _output_get 0.0 0.0) false false)))

(event OnComponentBeginOverlap(MagazineInsertCollision)
  (params (OverlappedComponent :type Primitive%20Component%20Object%20Reference) (OtherActor :type Actor%20Object%20Reference) (OtherComp :type Primitive%20Component%20Object%20Reference) (OtherBodyIndex :type Integer) (bFromSweep :type Boolean) (SweepResult :type Hit%20Result%20Structure%20%28by%20ref%29))
  (bind _asbp_magazine (Utilities|Casting|CastToBP_Magazine OtherActor))
  (if (Utilities|Enum|Equal(Enum) (Variables|/Game/Main/Blueprints/BP_Magazine.BP_Magazine_C|GetMagazineType _asbp_magazine) (Variables|Default|GetGunType))
    (if (Variables|/Game/VRTemplate/Blueprints/GripGrabComponent.GripGrabComponent_C|GetbIsHeld (Variables|/Game/Main/Blueprints/BP_Magazine.BP_Magazine_C|GetGrabComponent _asbp_magazine))
      (bind _output_get (Variables|Attachments|SetMagazine _asbp_magazine))
      (Default|PlayinSound _output_get)
      (Default|TryRelease (Variables|/Game/Main/Blueprints/BP_Magazine.BP_Magazine_C|GetGrabComponent _output_get))
      (EventDispatchers|BindEventtoOnGrabbed (Variables|/Game/Main/Blueprints/BP_Magazine.BP_Magazine_C|GetGrabComponent _output_get) (delegate Custom|TurnOnMagCollision))
      (Utilities|Time|SetTimerbyEvent (delegate Custom|AttachMagazine) 0.01 true))))

(event Custom|AttachMagazine
  (bind _returnvalue (Utilities|Time|GetWorldDeltaSeconds))
  (bind _magazine (Variables|Attachments|GetMagazine))
  (bind _magazinesnapspeedmultiplier (Variables|Functionality|GetMagazineSnapSpeedMultiplier))
  (bind _gunmesh (Variables|Default|GetGunMesh))
  (bind _returnvalue_2 (Transformation|GetSocketLocation _gunmesh "Magazine"))
  (bind _returnvalue_3 (* _returnvalue _magazinesnapspeedmultiplier))
  (bind _sm_handgun_magazine (Variables|/Game/Main/Blueprints/BP_Magazine.BP_Magazine_C|GetSM_Handgun_magazine _magazine))
  (bind _returnvalue_4 (Transformation|GetWorldLocation _sm_handgun_magazine))
  (bind _returnvalue_5 (Math|Interpolation|VInterpTo _returnvalue_4 _returnvalue_2 _returnvalue_3 1.0))
  (Transformation|SetRelativeLocation (Variables|/Script/Engine.Actor|GetRootComponent _magazine) _returnvalue_5 false false)
  (if (Utilities|Operators|EqualEqual _returnvalue_5 _returnvalue_2 0.01)
    (Transformation|AttachComponentToComponent (Variables|Attachments|GetMagazine) (Variables|Default|GetGunMesh) "Magazine" "SnapToTarget" "SnapToTarget" "KeepWorld" true)
    (Collision|SetCollisionResponsetoChannel (Variables|Default|GetMagazineInsertCollision) "ECC_GameTraceChannel3" "ECR_Ignore")
    (Class|KismetSystemLibrary|PauseTimer 0 "AttachMagazine")))

(event Custom|TurnOnMagCollision
  (params (Motion%20Controller :type Motion%20Controller%20Component%20Object%20Reference))
  (Collision|SetCollisionResponsetoChannel (Variables|Default|GetMagazineInsertCollision) "ECC_GameTraceChannel3" "ECR_Block")
  (Variables|Attachments|SetMagazine 0)
  (Development|PrintString "Mag Taken" true true "(R=1.000000,G=0.084230,B=0.000000,A=1.000000)"))

(event OnDropped(HandleGrabCompoonent)
  ;[1 0 0.1744] Trouble With Grabbing If Already Grabbed
  (Input|DisableInput (Game|GetPlayerController 0))
  (Input|RemoveMappingContext (PlayerController|LocalPlayerSubsystems|GetEnhancedInputLocalPlayerSubsystem (Game|GetPlayerController 0)) (select (Utilities|Enum|Equal(Enum) (Default|GetHeldbyHand (Variables|Default|GetHandleGrabCompoonent)) "Right") "/Game/VRTemplate/Input/IMC_Weapon_Right.IMC_Weapon_Right" "/Game/VRTemplate/Input/IMC_Weapon_Left.IMC_Weapon_Left") "(bIgnoreAllPressedKeysUntilRelease=True,bForceImmediately=False,bNotifyUserSettings=False)"))

(event OnGrabbed(HandleGrabCompoonent)
  (params (Motion%20Controller :type Motion%20Controller%20Component%20Object%20Reference))
  ;[1 0 0.1744] Trouble With Grabbing If Already Grabbed
  (Input|EnableInput (Game|GetPlayerController 0))
  (Input|AddMappingContext (PlayerController|LocalPlayerSubsystems|GetEnhancedInputLocalPlayerSubsystem (Game|GetPlayerController 0)) (select (Utilities|Enum|Equal(Enum) (Default|GetHeldbyHand (Variables|Default|GetHandleGrabCompoonent)) "Right") "/Game/VRTemplate/Input/IMC_Weapon_Right.IMC_Weapon_Right" "/Game/VRTemplate/Input/IMC_Weapon_Left.IMC_Weapon_Left") 0 "(bIgnoreAllPressedKeysUntilRelease=True,bForceImmediately=False,bNotifyUserSettings=False)"))

(event Input|EnhancedActionEvents|EnhancedInputActionIA_Shoot_Left
  (params (ActionValue :type Float%20%28double-precision%29) (ElapsedSeconds :type Float%20%28double-precision%29) (TriggeredSeconds :type Float%20%28double-precision%29) (InputAction :type Input%20Action%20Object%20Reference :default "/Game/VRTemplate/Input/Actions/IA_Shoot_Left.IA_Shoot_Left"))
  (bind (_location _direction) (GunFire|GunLocationandDirection 2e+05))
  (:Triggered
    (Variables|Default|SetActionValue_Left ActionValue)
    (Transformation|SetRelativeRotation (Variables|Default|GetTriggerMesh) (Math|Rotator|Lerp(Rotator) "0, 0, 0" (Variables|Functionality|GetTriggerFinalPossibleRotation) ActionValue) false false)
    (if (>= ActionValue (Variables|Firing|GetTriggerFireThreshold))
      (Utilities|FlowControl|DoOnce false :!label _label
        (:Completed
          (Variables|Attachments|GetMagazine
            (:then
              (if (Variables|SlideVariables|GetChamberHasBullet)
                (if (Variables|/Game/Main/Blueprints/BP_Magazine.BP_Magazine_C|GetIsEmpty (Variables|Attachments|GetMagazine))
                  (|PlaySlideAnimation :!label _label_2
                    (:LastBulletAnimationDone
                      (Rendering|SetVisibility (Variables|Default|GetRoundMesh) false false)
                      (Variables|SlideVariables|SetChamberHasBullet false))
                    (:FullSlideAnimationDone
                      (GunFire|LineTracefromBarrel _location _direction)))
                  (else
                    (goto _label_2 FullSlideFireAnimation)))
                (else
                  (if (Variables|SlideVariables|GetDryFire) :!label _label_3
                    (Audio|PlaySoundatLocation (Variables|Sounds|GetDryFireRoundSound) (Transformation|GetWorldLocation (Variables|Default|GetTriggerMesh)) "0, 0, 0" 1.0 1.0 0.0 0 0 0 0)
                    (Variables|SlideVariables|SetDryFire false)
                    (else
                      (Audio|PlaySoundatLocation (Variables|Sounds|GetEmptyTriggerSound) (Transformation|GetWorldLocation (Variables|Default|GetTriggerMesh)) "0, 0, 0" 1.0 1.0 0.0 0 0 0 0))))))
            (:else
              (if (Variables|SlideVariables|GetChamberHasBullet)
                (goto _label_2)
                (else
                  (goto _label_3)))))))
      (else
        (goto _label Reset))))
  (:Canceled
    (Variables|Default|SetActionValue_Left 0.0 :!label _label_4)
    (goto _label Reset))
  (:Completed
    (goto _label_4)))

(event Input|EnhancedActionEvents|EnhancedInputActionIA_Shoot_Right
  (params (ActionValue :type Float%20%28double-precision%29) (ElapsedSeconds :type Float%20%28double-precision%29) (TriggeredSeconds :type Float%20%28double-precision%29) (InputAction :type Input%20Action%20Object%20Reference :default "/Game/VRTemplate/Input/Actions/IA_Shoot_Right.IA_Shoot_Right"))
  (bind (_location _direction) (GunFire|GunLocationandDirection 2e+05))
  (:Triggered
    (Variables|Default|SetActionValue_Left ActionValue)
    (Transformation|SetRelativeRotation (Variables|Default|GetTriggerMesh) (Math|Rotator|Lerp(Rotator) "0, 0, 0" (Variables|Functionality|GetTriggerFinalPossibleRotation) ActionValue) false false)
    (if (>= ActionValue (Variables|Firing|GetTriggerFireThreshold))
      (Utilities|FlowControl|DoOnce false :!label _label
        (:Completed
          (Variables|Attachments|GetMagazine
            (:then
              (if (Variables|SlideVariables|GetChamberHasBullet)
                (if (Variables|/Game/Main/Blueprints/BP_Magazine.BP_Magazine_C|GetIsEmpty (Variables|Attachments|GetMagazine))
                  (|PlaySlideAnimation :!label _label_2
                    (:LastBulletAnimationDone
                      (Rendering|SetVisibility (Variables|Default|GetRoundMesh) false false)
                      (Variables|SlideVariables|SetChamberHasBullet false))
                    (:FullSlideAnimationDone
                      (GunFire|LineTracefromBarrel _location _direction)))
                  (else
                    (goto _label_2 FullSlideFireAnimation)))
                (else
                  (if (Variables|SlideVariables|GetDryFire) :!label _label_3
                    (Audio|PlaySoundatLocation (Variables|Sounds|GetDryFireRoundSound) (Transformation|GetWorldLocation (Variables|Default|GetTriggerMesh)) "0, 0, 0" 1.0 1.0 0.0 0 0 0 0)
                    (Variables|SlideVariables|SetDryFire false)
                    (else
                      (Audio|PlaySoundatLocation (Variables|Sounds|GetEmptyTriggerSound) (Transformation|GetWorldLocation (Variables|Default|GetTriggerMesh)) "0, 0, 0" 1.0 1.0 0.0 0 0 0 0))))))
            (:else
              (if (Variables|SlideVariables|GetChamberHasBullet)
                (goto _label_2)
                (else
                  (goto _label_3)))))))
      (else
        (goto _label Reset))))
  (:Canceled
    (Variables|Default|SetActionValue_Left 0.0 :!label _label_4)
    (goto _label Reset))
  (:Completed
    (goto _label_4)))

(event Custom|EjectBullet)

(fn ConstructionScript)

(fn PlaySoundatLocation
  (params (Location :type Vector) (SoundCue :type Sound%20Cue%20Object%20Reference))
  (Audio|PlaySoundatLocation SoundCue Location "0, 0, 0" 1.0 1.0 0.0 0 0 0 0))

(fn GetGrabOffsetBetweenMC&SlideCurl
  (return (- (Transformation|GetWorldLocation (Variables|/Game/VRTemplate/Blueprints/CurlGrabComponent.CurlGrabComponent_C|GetMotionControllerRef (Variables|Default|GetCurlGrabComponent))) (Transformation|GetWorldLocation (Variables|Default|GetSlideMesh)))))

(fn ClampSlideMovementCurl
  (params (Min :type Float%20%28double-precision%29))
  (return (Math|Float|Clamp(Float) (+ (.x (Math|Transform|InverseTransformLocation (Transformation|GetWorldTransform (Variables|Default|GetSlideMesh)) (- (Transformation|GetWorldLocation (Variables|/Game/VRTemplate/Blueprints/CurlGrabComponent.CurlGrabComponent_C|GetMotionControllerRef (Variables|Default|GetCurlGrabComponent))) (Variables|SlideVariables|GetInitialGrabOffset)))) (.x (Variables|/Script/Engine.SceneComponent|GetRelativeLocation (Variables|Default|GetSlideMesh)))) Min 0.0)))

(fn GetGrabOffsetBetweenMC&SlideDefault
  (return (- (Transformation|GetWorldLocation (Variables|/Game/VRTemplate/Blueprints/GripGrabComponent.GripGrabComponent_C|GetMotionControllerRef (Variables|Default|GetGripGrabComponent))) (Transformation|GetWorldLocation (Variables|Default|GetSlideMesh)))))

(fn ClampSlideMovementDefault
  (params (Min :type Float%20%28double-precision%29))
  (return (Math|Float|Clamp(Float) (+ (.x (Math|Transform|InverseTransformLocation (Transformation|GetWorldTransform (Variables|Default|GetSlideMesh)) (- (Transformation|GetWorldLocation (Variables|/Game/VRTemplate/Blueprints/GripGrabComponent.GripGrabComponent_C|GetMotionControllerRef (Variables|Default|GetGripGrabComponent))) (Variables|SlideVariables|GetInitialGrabOffset)))) (.x (Variables|/Script/Engine.SceneComponent|GetRelativeLocation (Variables|Default|GetSlideMesh)))) Min 0.0)))

(fn GunLocationandDirection
  (params (Distance :type Float%20%28double-precision%29))
  (bind _silenserattached_ (Variables|Attachments|GetSilenserAttached?))
  (bind _gunmesh (Variables|Default|GetGunMesh))
  (bind _returnvalue (Transformation|GetSocketLocation _gunmesh "SilencerBarrel"))
  (bind _returnvalue_2 (Transformation|GetSocketLocation _gunmesh "Barrel"))
  (bind _returnvalue_3 (select _silenserattached_ _returnvalue _returnvalue_2))
  (return _returnvalue_3 (+ _returnvalue_3 (* (Math|Vector|GetForwardVector (Transformation|GetSocketRotation _gunmesh "Barrel")) Distance))))

(fn LineTracefromBarrel
  (params (Trace%20start%20location :type Vector) (Trace%20end%20location :type Vector))
  (bind _outhit (Collision|LineTraceByChannel Trace%20start%20location Trace%20end%20location "TraceTypeQuery1" false 0 "ForDuration" true "(R=1.000000,G=0.000000,B=0.000000,A=1.000000)" "(R=0.000000,G=1.000000,B=0.000000,A=1.000000)" 4.0))
  (return _outhit))