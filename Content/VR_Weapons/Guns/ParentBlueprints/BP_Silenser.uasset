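; Silencer attachment actor for VR guns.
; On BeginPlay it puts GrabBounds into finger-curl collision mode by blocking one custom trace channel and ignoring another.
; A matching helper swaps those two channel responses for grab mode, though nothing in this graph calls it.
; A separate function plays the attach sound at the GunCollision component's location.
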(event EventBeginPlay
  (CallFunction|SetCollisionforCurl (Variables|Default|GetGrabBounds)))

(event Collision|EventActorBeginOverlap
  (params (OtherActor :type Actor%20Object%20Reference)))

(event EventTick
  (params (DeltaSeconds :type Float%20%28single-precision%29)))

(fn ConstructionScript)

(fn PlayAttachmentSound
  (Audio|PlaySoundatLocation (Variables|Default|GetSilenserAttachSoundCue) (Transformation|GetWorldLocation (Variables|Default|GetGunCollision)) "0, 0, 0" 1.0 1.0 0.0 0 0 0 0))

(fn SetCollisionforCurl
  (params (CollisionComp :type Primitive%20Component%20Object%20Reference))
  (Collision|SetCollisionResponsetoChannel CollisionComp "ECC_GameTraceChannel6" "ECR_Block")
  (Collision|SetCollisionResponsetoChannel CollisionComp "ECC_GameTraceChannel4" "ECR_Ignore"))

(fn SetCollisionforGrab
  (params (CollisionComp :type Primitive%20Component%20Object%20Reference))
  (Collision|SetCollisionResponsetoChannel CollisionComp "ECC_GameTraceChannel4" "ECR_Block")
  (Collision|SetCollisionResponsetoChannel CollisionComp "ECC_GameTraceChannel6" "ECR_Ignore"))