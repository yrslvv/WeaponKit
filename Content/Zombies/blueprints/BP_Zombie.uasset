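; Zombie actor that takes bone-based bullet damage, reacts physically to hits and ragdolls on death.
; BulletDamage applies seeded random head or body damage, or mass-based limb damage, and multicasts health to a player-facing health bar.
; Surviving hits blend physics below the struck bone through a Timeline weight applied on Tick, plus an impulse.
; Lethal hits simulate the whole mesh, break head or limb constraints and flag the anim Blueprint dead.
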(event EventBeginPlay)

(event Collision|EventActorBeginOverlap
  (params (OtherActor :type Actor%20Object%20Reference)))

(event EventTick
  (params (DeltaSeconds :type Float%20%28single-precision%29))
  (CallFunction|RotateHealthBar)
  (|Updatephysicsbodies_2))

(event EventBulletDamage
  (params (Random%20seed :type Integer) (Bone :type Name :default "None") (Impulse :type Vector :default "0, 0, 0") (Damage%20multiplier :type Float%20%28double-precision%29) (Dismemeber :type Boolean) (Instigator :type Pawn%20Object%20Reference))
  (bind _mesh (Variables|Character|GetMesh))
  (if (and (not (Variables|Default|GetIsDead)) (!= Bone ""))
    (Game|Damage|ApplyDamage Bone Damage%20multiplier Random%20seed)
    (|Setvariables Bone Impulse)
    ;[0 0 0] Check health level
    (Utilities|FlowControl|Delay 0.02)
    (if (> (Variables|Default|GetHealth) 0.0)
      (Class|AISenseDamage|ReportDamageEvent self (Game|Player|GetPlayerPawn 0) 0.0 (Transformation|GetActorLocation) "0, 0, 0" "None")
      (|Validbonehit_2
        (:True
          (Utilities|FlowControl|Sequence
            (:then_0
              (|AnimateBlendWeight_2))
            (:then_1
              (|Hitbonephysicsimpulse_2)))))
      (else
        (Variables|Default|SetIsDead false)
        (Variables|Default|SetBlendWeight 0.0)
        (Utilities|FlowControl|Delay 0.06)
        (if (Utilities|Name|NotEqual(Name) (Variables|Default|GetBoneName) "Hips") ; don't apply physics impulse to root bone
          (Class|SkeletalMeshComponent|SetAllBodiesSimulatePhysics (Variables|Character|GetMesh) true) ; simulate physics on death
          (Physics|AddImpulse _mesh (* (Variables|Default|GetImpulse) 0.3) (Variables|Default|GetBoneName) true)
          (CallFunction|DismemberBodyPart)
          (else
            (Class|SkeletalMeshComponent|SetAllBodiesSimulatePhysics (Variables|Character|GetMesh) true) ; simulate physics on death
          ))
        (Class|PrimitiveComponent|SetNotifyRigidBodyCollision _mesh false) ; disable additional physics impulses once killed
        (bind _aszombie_anim_bp (Utilities|Casting|CastToZombieAnimBP (Components|SkeletalMesh|GetAnimInstance (Variables|Character|GetMesh))))
        (Variables|/Game/Zombies/ZombieAnimBP.ZombieAnimBP_C|SetIsDead _aszombie_anim_bp true)))))

(fn ConstructionScript)

(fn GetDamageBasedonBoneHit
  (params (BoneName :type Name) (Damage%20mulitply :type Float%20%28double-precision%29) (InitialSeed :type Integer))
  (bind _returnvalue (Math|Random|MakeRandomStream InitialSeed))
  (LocalVariables|SetBone BoneName)
  (LocalVariables|SetDamage%20mulitplier Damage%20mulitply)
  (LocalVariables|SetHeadshot%20damage (Math|Random|RandomFloatinRangefromStream _returnvalue 3e+01 4e+01))
  (LocalVariables|SetBodyshot%20damage (Math|Random|RandomFloatinRangefromStream _returnvalue 5.0 15.0))
  (return (* (LocalVariables|GetDamage%20mulitplier) (Math|Float|SelectFloat (LocalVariables|GetHeadshot%20damage) (Math|Float|SelectFloat (* (Class|SkeletalMeshComponent|GetBoneMass (Variables|Character|GetMesh) (LocalVariables|GetBone) true) 1.0) (LocalVariables|GetBodyshot%20damage) (CallFunction|LimbHit (LocalVariables|GetBone))) (CallFunction|Headshot (LocalVariables|GetBone))))))

(fn Headshot
  (params (BoneName :type Name))
  (return (Class|SkinnedMeshComponent|BoneIsChildOf (Variables|Character|GetMesh) BoneName "Neck")))

(fn LimbHit
  (params (Bone :type Name))
  (bind _mesh (Variables|Character|GetMesh))
  (return (Math|Boolean|ORBoolean (or (Class|SkinnedMeshComponent|BoneIsChildOf _mesh Bone "LeftArm") (Utilities|Name|Equal(Name) Bone "LeftArm")) (or (Class|SkinnedMeshComponent|BoneIsChildOf _mesh Bone "RightArm") (Utilities|Name|Equal(Name) Bone "RightArm")) (or (Class|SkinnedMeshComponent|BoneIsChildOf _mesh Bone "RightUpLeg") (Utilities|Name|Equal(Name) Bone "RightUpLeg")) (or (Class|SkinnedMeshComponent|BoneIsChildOf _mesh Bone "LeftUpLeg") (Utilities|Name|Equal(Name) Bone "LeftUpLeg")))))

(fn RotateHealthBar
  (bind _returnvalue (Game|Player|GetPlayerPawn 0))
  (bind _healthbar (Variables|Default|GetHealthBar))
  (bind _returnvalue_2 (Transformation|GetWorldRotation _healthbar))
  (Utilities|IsValid _returnvalue
    (:Is%20Valid
      (Transformation|SetWorldRotation (Variables|Default|GetHealthBar) (Math|Rotator|MakeRotator (.roll _returnvalue_2) (.pitch _returnvalue_2) (Math|Interpolation|FInterpTo (.yaw _returnvalue_2) (.yaw (Math|Rotator|FindLookatRotation (Transformation|GetWorldLocation _healthbar) (Transformation|GetActorLocation _returnvalue))) (Utilities|Time|GetWorldDeltaSeconds) 3.0)) false false))))

(fn DismemberBodyPart
  (bind _bonename (Variables|Default|GetBoneName))
  (if (or (CallFunction|Headshot _bonename) (CallFunction|LimbHit _bonename))
    (Class|SkeletalMeshComponent|BreakConstraint (Variables|Character|GetMesh) (* (Variables|Default|GetImpulse) 0.6) "0, 0, 0" (Variables|Default|GetBoneName)))
  (return))

(event Custom|Multicast%20update%20healthbar
  ;[0.494 0.3303 1] Update health  bar
  (bind _aswidget_health_bar (Utilities|Casting|CastToWidget_HealthBar (UserInterface|GetUserWidgetObject (Variables|Default|GetHealthBar))))
  (Default|UpdateHealth _aswidget_health_bar (Variables|Default|GetHealth)))